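; BP_lapPointPlacer places BP_lapPoint actors along a spline, apparently as lap markers for a track.
; Its placePoint event first destroys and clears the previously stored points in AllPoint, so each call rebuilds the set.
; It then spawns points at world transforms sampled by spline time from index over PointAmount, storing each in AllPoint.
; The construction script is empty, so placement happens only through that event.
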(event Custom|placePoint
  (bind _allpoint (Variables|Default|GetallPoint))
  (bind _pointamount (Variables|Default|GetpointAmount))
  (Utilities|FlowControl|Sequence
    (:then_0
      (for _array_element _allpoint
        (Actor|DestroyActor _array_element))
      (Utilities|Array|Clear _allpoint))
    (:then_1
      (for _index (range 0 _pointamount)
        (bind _returnvalue (Game|SpawnActorfromClass "/Game/blueprint/lap/BP_lapPoint.BP_lapPoint_C" (Spline|GetTransformatTime (Variables|Default|GetSpline) (/ _index _pointamount) "World" false false) "Undefined" "MultiplyWithRoot" 0 0))
        (Utilities|Array|Add (Variables|Default|GetallPoint) _returnvalue)))))

(fn ConstructionScript)
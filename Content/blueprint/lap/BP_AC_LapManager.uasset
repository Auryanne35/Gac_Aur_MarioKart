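; BP_AC_LapManager tracks lap progress in a race, counting laps and detecting the finish.
; AddLapPoint records unique checkpoints, and AddLap only counts a lap when at least 75% of the game mode's lap points are crossed, or on lap zero.
; Each counted lap clears the checkpoints and fires OnLapAdded.
; Exceeding the game mode's lap count calls FinishRace, which currently only prints a message.
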(event EventBeginPlay)

(event EventTick
  (params (DeltaSeconds :type Float%20%28single-precision%29)))

(fn AddLap
  (if (or (>= (Utilities|Array|Length (Variables|Default|GetlapPointCrossed)) (* (Variables|/Game/baseUnreal/VehicleTemplate/Blueprints/BP_VehicleAdvGameMode.BP_VehicleAdvGameMode_C|GetLapPointNumber (CallFunction|GetMKGameMode)) 0.75)) (== (Variables|Default|GetcurrentLap) 0))
    (Utilities|Array|Clear (Variables|Default|GetlapPointCrossed))
    (bind _output_get (Variables|Default|SetcurrentLap (+ (Variables|Default|GetcurrentLap) 1)))
    (Default|CallOnLapAdded (Variables|Default|GetcurrentLap))
    (if (> _output_get (Variables|/Game/baseUnreal/VehicleTemplate/Blueprints/BP_VehicleAdvGameMode.BP_VehicleAdvGameMode_C|GetnumberOfLap (CallFunction|GetMKGameMode)))
      (CallFunction|FinishRace))))

(fn FinishRace
  (Development|PrintString "finish"))

(fn AddLapPoint
  (params (lapPoint :type BP%20Lap%20Point%20Object%20Reference%20%28by%20ref%29))
  (Utilities|Array|AddUnique (Variables|Default|GetlapPointCrossed) lapPoint))
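; BP_couleur is an actor whose sphere changes to a random color each time a looping timeline completes.
; On BeginPlay it creates a dynamic material instance from M_couleur and assigns it to the Sphere component.
; The Timeline serves as a repeating timer: its Finished output writes random RGBA values to the "Color" vector parameter, then restarts it from the beginning.
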(event EventBeginPlay
  (bind _returnvalue (Rendering|Material|CreateDynamicMaterialInstance "/Game/blueprint/M_couleur.M_couleur" "None" "None" :!class /Script/Engine.KismetMaterialLibrary))
  (bind _output_get (Variables|Default|SetmaterialColor _returnvalue))
  (Rendering|Material|SetMaterial (Variables|Default|GetSphere) 0 _output_get)
  (Timeline|Timeline Play
    (:Finished
      (Rendering|Material|SetVectorParameterValue (Variables|Default|GetmaterialColor) "Color" (Math|Color|MakeColor (Math|Random|RandomFloat) (Math|Random|RandomFloat) (Math|Random|RandomFloat) (Math|Random|RandomFloat)) :!class /Script/Engine.MaterialInstanceDynamic)
      (Timeline|Timeline PlayFromStart))))

(event Collision|EventActorBeginOverlap
  (params (OtherActor :type Actor%20Object%20Reference)))

(event EventTick
  (params (DeltaSeconds :type Float%20%28single-precision%29)))

(fn ConstructionScript)
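; BP_itemBox is a pickup box that gives a random item to a vehicle that drives into it.
; When the Cube overlaps a BP_VehicleAdvPawnBase, it picks a random entry from ListObject and passes it to GetItem on the object returned by GetCastedControlled.
; The box then hides and disables collision for a few seconds before reappearing with query-only collision.
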(event OnComponentBeginOverlap(Cube)
  (params (OverlappedComponent :type Primitive%20Component%20Object%20Reference) (OtherActor :type Actor%20Object%20Reference) (OtherComp :type Primitive%20Component%20Object%20Reference) (OtherBodyIndex :type Integer) (bFromSweep :type Boolean) (SweepResult :type Hit%20Result%20Structure%20%28by%20ref%29))
  (bind _asbp_vehicle_adv_pawn_base (Utilities|Casting|CastToBP_VehicleAdvPawnBase OtherActor))
  (bind _asbp_vehicle_adv_player_controller (Default|GetCastedControlled _asbp_vehicle_adv_pawn_base))
  (bind _item (CallFunction|GetRandomItem))
  (Default|GetItem _asbp_vehicle_adv_player_controller _item)
  (CallFunction|Disapear))

(event Custom|disapear
  (bind _cube (Variables|Default|GetCube))
  (bind _cube_2 (Variables|Default|GetCube))
  (Rendering|SetVisibility _cube_2 false false)
  (Collision|SetCollisionEnabled _cube_2 "NoCollision")
  (Utilities|FlowControl|Delay 3.0)
  (Rendering|SetVisibility _cube true false)
  (Collision|SetCollisionEnabled _cube "QueryOnly"))

(event EventBeginPlay)

(event Collision|EventActorBeginOverlap
  (params (OtherActor :type Actor%20Object%20Reference)))

(event EventTick
  (params (DeltaSeconds :type Float%20%28single-precision%29)))

(fn ConstructionScript)

(fn GetRandomItem
  (bind _listobject (Variables|Default|GetlistObject))
  (return (Utilities|Array|Get(acopy) _listobject (Math|Random|RandomIntegerinRange 0 (- (Utilities|Array|Length _listobject) 1)))))